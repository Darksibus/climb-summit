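; VR backpack actor that attaches to the player character and stores objects held in the motion controllers.
; Right grip detaches the pack, or snaps it to the attachment point and parents it to the camera.
; Releasing either grip over the pack plays a shared timeline shrinking held objects, then links them to the pack mesh.
; Gripping while overlapping a linked object detaches it.
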(event `Key|MotionController_Right_Grip1`
  (params (Key :type "Key Structure"))
  (:`Pressed`
    (bind _returnvalue (`PrimitiveComponent.IsOverlappingComponent` (`/Game/Blueprints/Character_Blueprint.GrabSphereR` (stale `Key|MotionController_Right_Grip1` _ascharacter_blueprint)) (`/Game/Blueprints/Character_Blueprint.PackCollision` (stale `Key|MotionController_Right_Grip1` _ascharacter_blueprint))))
    (if _returnvalue
      (`self.K2_DetachFromActor` "KeepRelative")))
  (:`Released`
    (bind _ascharacter_blueprint (cast `/Game/Blueprints/Character_Blueprint` (`self.GetOwner`)))
    (if (`/Game/Blueprints/Character_Blueprint.HeldR` _ascharacter_blueprint)
      (if _returnvalue
        (`self.K2_SetActorTransform` (`KismetMathLibrary.Conv_VectorToTransform` (`SceneComponent.K2_GetComponentLocation` (`/Game/Blueprints/Character_Blueprint.PackAttachmentPoint` _ascharacter_blueprint))))
        (`self.K2_AttachToComponent` (`/Game/Blueprints/Character_Blueprint.Camera` _ascharacter_blueprint) "None" "KeepRelative" "KeepRelative" "KeepRelative")))))

(event `Key|MotionController_Right_Grip1`
  (params (Key :type "Key Structure"))
  (bind _packsm (`self.PackSM`))
  (:`Pressed`
    (if (stale `Key|MotionController_Right_Grip1` _returnvalue_4)
      (if (`PrimitiveComponent.IsOverlappingComponent` (stale _asprimitive_component) (`/Game/Blueprints/Character_Blueprint.GrabSphereR` (stale `Key|MotionController_Right_Grip1` _ascharacter_blueprint)))
        (`SceneComponent.K2_DetachFromComponent` (stale _asprimitive_component) "KeepRelative" "KeepRelative" "KeepRelative" true))))
  (:`Released`
    (if (and (`/Game/Blueprints/Character_Blueprint.HeldR` (stale `Key|MotionController_Right_Grip1` _ascharacter_blueprint)) (`PrimitiveComponent.IsOverlappingComponent` (`self.PackCollision`) (`/Game/Blueprints/Character_Blueprint.GrabSphereR` (stale `Key|MotionController_Right_Grip1` _ascharacter_blueprint))))
      (bind _asprimitive_component (cast `PrimitiveComponent` (`/Game/Blueprints/Character_Blueprint.HeldObjectR` (stale `Key|MotionController_Right_Grip1` _ascharacter_blueprint))))
      (if (`PrimitiveComponent.IsOverlappingComponent` (`self.PackCollision`) _asprimitive_component)
        (bind (_direction _alpha_lerp) (`Timeline|LerpTimeline` :!via `PlayFromStart` :!label _label)
          (:`Update`
            (`|ExecutionSequence`
              (:`then_0`
                (bind _returnvalue (`SceneComponent.K2_GetComponentLocation` _asprimitive_component))
                (bind _returnvalue_2 (`SceneComponent.K2_GetComponentLocation` (`/Game/Blueprints/Character_Blueprint.PackAttachmentPoint` (stale `Key|MotionController_Right_Grip1` _ascharacter_blueprint))))
                (`SceneComponent.K2_SetRelativeTransform` _asprimitive_component (`KismetMathLibrary.TLerp` (`KismetMathLibrary.Conv_VectorToTransform` _returnvalue) (`KismetMathLibrary.MakeTransform` (- _returnvalue _returnvalue_2) (struct) (0.1 0.1 0.1)) _alpha_lerp) false false))
              (:`then_1`
                (bind _returnvalue_3 (`SceneComponent.K2_GetComponentLocation` (stale _asprimitive_component)))
                (`SceneComponent.K2_SetRelativeTransform` (stale _asprimitive_component) (`KismetMathLibrary.TLerp` (`KismetMathLibrary.Conv_VectorToTransform` _returnvalue_3) (`KismetMathLibrary.MakeTransform` (- _returnvalue_3 _returnvalue_2) (struct) (0.1 0.1 0.1)) _alpha_lerp) false false))))
          (:`Finished`
            (`|ExecutionSequence`
              (:`then_0`
                (bind _returnvalue_4 (`SceneComponent.K2_AttachToComponent` _packsm _asprimitive_component "None" "KeepRelative" "KeepRelative" "KeepRelative" true)))
              (:`then_1`
                (`SceneComponent.K2_AttachToComponent` (stale _asprimitive_component) _packsm "None" "KeepRelative" "KeepRelative" "KeepRelative" true)))))))))

(event `Key|MotionController_Left_Grip1`
  (params (Key :type "Key Structure"))
  (:`Pressed`
    (if (stale `Key|MotionController_Right_Grip1` _returnvalue_4)
      (if (`PrimitiveComponent.IsOverlappingComponent` (stale _asprimitive_component) (`/Game/Blueprints/Character_Blueprint.GrabSphereL` (stale `Key|MotionController_Right_Grip1` _ascharacter_blueprint)))
        (`SceneComponent.K2_DetachFromComponent` (stale _asprimitive_component) "KeepRelative" "KeepRelative" "KeepRelative" true))))
  (:`Released`
    (if (and (`/Game/Blueprints/Character_Blueprint.HeldL` (stale `Key|MotionController_Right_Grip1` _ascharacter_blueprint)) (`PrimitiveComponent.IsOverlappingComponent` (`self.PackCollision`) (`/Game/Blueprints/Character_Blueprint.GrabSphereR` (stale `Key|MotionController_Right_Grip1` _ascharacter_blueprint))))
      (bind _asprimitive_component (cast `PrimitiveComponent` (`/Game/Blueprints/Character_Blueprint.HeldObjectL` (stale `Key|MotionController_Right_Grip1` _ascharacter_blueprint))))
      (if (`PrimitiveComponent.IsOverlappingComponent` (`self.PackCollision`) _asprimitive_component)
        (goto _label :!via `PlayFromStart`)))))

(fn `UserConstructionScript`)