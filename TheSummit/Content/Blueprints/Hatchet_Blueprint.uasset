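; Hatchet weapon Blueprint that damages actors its mesh overlaps while it is moving.
; Tick records the mesh's world location through a short Delay, giving a slightly stale reference position.
; On overlap, damage applies only if the mesh has moved far enough from that position, a simple swing-speed check.
; After a hit, it briefly disables the mesh component's tick, which does not itself gate the overlap event.
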(event `self.ReceiveTick`
  (params (DeltaSeconds :type "Float (single-precision)"))
  (`KismetSystemLibrary.Delay` 0.1)
  (bind _output_get (set `self.oldLocation` (`SceneComponent.K2_GetComponentLocation` (`self.StaticMeshComponent`)))))

(event `self.StaticMeshComponent.OnComponentBeginOverlap`
  (params (OverlappedComponent :type "PrimitiveComponent Object Reference") (OtherActor :type "Actor Object Reference") (OtherComp :type "PrimitiveComponent Object Reference") (OtherBodyIndex :type Integer) (bFromSweep :type Boolean) (SweepResult :type "HitResult Structure (by ref)"))
  (bind _staticmeshcomponent (`self.StaticMeshComponent`))
  (if (>= (`KismetMathLibrary.VSize` (- (`SceneComponent.K2_GetComponentLocation` (`self.StaticMeshComponent`)) (stale `self.ReceiveTick` _output_get))) 5.0)
    (`GameplayStatics.ApplyDamage` OtherActor 1.0)
    (`ActorComponent.SetComponentTickEnabled` _staticmeshcomponent false)
    (`KismetSystemLibrary.Delay` 0.5)
    (`ActorComponent.SetComponentTickEnabled` _staticmeshcomponent true)))

(fn `UserConstructionScript`)