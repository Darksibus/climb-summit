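; Tree actor that can be felled to yield a wood item.
; Pressing F applies one point of damage to the tree's own actor, with no range or target check in the graph.
; Damage lowers Health, and at zero or below the tree spawns WoodItem_Blueprint slightly below its mesh origin, turns off shadow casting and destroys itself.
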(event `Key|F`
  (params (Key :type "Key Structure"))
  (:`Pressed`
    (`GameplayStatics.ApplyDamage` (`ActorComponent.GetOwner` (`self.StaticMeshComponent`)) 1.0)))

(event `self.ReceiveAnyDamage`
  (params (Damage :type "Float (single-precision)") (DamageType :type "DamageType Object Reference") (InstigatedBy :type "Controller Object Reference") (DamageCauser :type "Actor Object Reference"))
  (bind _staticmeshcomponent (`self.StaticMeshComponent`))
  (bind _output_get (set `self.health` (- (`self.health`) Damage)))
  (if (<= _output_get 0.0)
    (`|SpawnActorFromClass` "/Game/Blueprints/WoodItem_Blueprint.WoodItem_Blueprint_C" (`KismetMathLibrary.Conv_VectorToTransform` (- (`SceneComponent.K2_GetComponentLocation` _staticmeshcomponent) (* (`SceneComponent.GetUpVector` _staticmeshcomponent) 2))) "AlwaysSpawn" "OverrideRootScale" null null)
    (`PrimitiveComponent.SetCastShadow` _staticmeshcomponent false)
    (`self.K2_DestroyActor`)))

(fn `UserConstructionScript`)