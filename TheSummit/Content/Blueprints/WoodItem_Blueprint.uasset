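; Wood pickup actor that merges with other wood items into a counted stack.
; When WoodMesh overlaps another wood item, it destroys that actor and increments AmountOfWood.
; When either character grab sphere overlaps StackCollision, the text shows the count, then a non-empty stack spawns a wood item at the mesh, attaches it to the mesh's parent and decrements the count.
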(event `self.WoodMesh.OnComponentBeginOverlap`
  (params (OverlappedComponent :type "PrimitiveComponent Object Reference") (OtherActor :type "Actor Object Reference") (OtherComp :type "PrimitiveComponent Object Reference") (OtherBodyIndex :type Integer) (bFromSweep :type Boolean) (SweepResult :type "HitResult Structure (by ref)"))
  ;[1 1 1] Increment amount of wood
  (bind _aswood_item_blueprint (cast `/Game/Blueprints/WoodItem_Blueprint` OtherActor))
  (`self.K2_DestroyActor` _aswood_item_blueprint)
  (bind _result (`/Engine/EditorBlueprintResources/StandardMacros.IncrementInt` (`self.AmountOfWood`))
    (:`  `
      (set `self.AmountOfWood` _result))))

(event `self.StackCollision.OnComponentBeginOverlap`
  (params (OverlappedComponent :type "PrimitiveComponent Object Reference") (OtherActor :type "Actor Object Reference") (OtherComp :type "PrimitiveComponent Object Reference") (OtherBodyIndex :type Integer) (bFromSweep :type Boolean) (SweepResult :type "HitResult Structure (by ref)"))
  (bind _woodmesh (`self.WoodMesh`))
  (bind _amountofwood (`self.AmountOfWood`))
  ;[1 1 1] Display amount of wood in stack
  (bind _ascharacter_blueprint (cast `/Game/Blueprints/Character_Blueprint` OtherActor))
  (if (or (== (`/Game/Blueprints/Character_Blueprint.GrabSphereL` _ascharacter_blueprint) OtherComp) (== (`/Game/Blueprints/Character_Blueprint.GrabSphereR` _ascharacter_blueprint) OtherComp))
    (`TextRenderComponent.K2_SetText` (`self.TextRender`) (`KismetTextLibrary.Conv_IntToText` _amountofwood))
    ;[1 1 1] Stacking physics
    (if (> _amountofwood 0)
      (bind _returnvalue (`|SpawnActorFromClass` "WoodItem_Blueprint_C" (`KismetMathLibrary.Conv_VectorToTransform` (`SceneComponent.K2_GetComponentLocation` _woodmesh)) "AlwaysSpawn" "OverrideRootScale" null null))
      (`self.K2_AttachToComponent` _returnvalue (`SceneComponent.GetAttachParent` _woodmesh) "None" "KeepRelative" "KeepRelative" "KeepRelative" true)
      (set `self.AmountOfWood` (- (`self.AmountOfWood`) 1)))))

(fn `UserConstructionScript`)