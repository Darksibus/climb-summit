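; VR hand Blueprint that lets the right motion controller grab nearby actors with its grip button.
; The grip press calls GrabActor, which picks the closest interface-implementing actor overlapping GrabSphere and snaps it onto RightHand.
; ReleaseActor detaches the held actor only if still parented to MCRightHand, but no event in this graph calls it.
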(event `Key|MotionController_Right_Grip1`
  (params (Key :type "Key Structure"))
  (:`Pressed`
    (`self.GrabActor`)))

(fn `GetActorNearHand`
  (returns (NearestMesh :type "Actor Object Reference"))
  (locals (NearestOverlappingActor :type "Actor Object Reference") (NearestOverlap :type "Float (double-precision)"))
  (bind _grabsphere (`self.GrabSphere`))
  (for _array_element (`PrimitiveComponent.GetOverlappingActors` _grabsphere "/Script/Engine.Actor")
    (if (`KismetSystemLibrary.DoesImplementInterface` _array_element)
      (bind _returnvalue (`KismetMathLibrary.VSize` (- (`self.K2_GetActorLocation` _array_element) (`SceneComponent.K2_GetComponentLocation` _grabsphere))))
      (if (< _returnvalue (`local.NearestOverlap`))
        (set `local.NearestOverlappingActor` _array_element)
        (set `local.NearestOverlap` _returnvalue))))
  (return (`local.NearestOverlappingActor`)))

(fn `GrabActor`
  (set `self.WantsToGrip` true)
  (bind _nearestmesh (`self.GetActorNearHand`))
  (`/Engine/EditorBlueprintResources/StandardMacros.IsValid` _nearestmesh
    (:`Is Valid`
      (set `self.AttachedActor` _nearestmesh)
      (`self.K2_AttachToComponent` _nearestmesh (`self.RightHand`) "None" "SnapToTarget" "SnapToTarget" "KeepRelative" true))))

(fn `ReleaseActor`
  (bind _attachedactor (`self.AttachedActor`))
  (set `self.WantsToGrip` false)
  (`/Engine/EditorBlueprintResources/StandardMacros.IsValid` _attachedactor
    (:`Is Valid`
      (if (== (`SceneComponent.GetAttachParent` (`self.K2_GetRootComponent` _attachedactor)) (`self.MC_RightHand`))
        (`self.K2_DetachFromActor` _attachedactor "KeepWorld" "KeepWorld" "KeepWorld"))
      (set `self.AttachedActor` null))))

(fn `UserConstructionScript`)