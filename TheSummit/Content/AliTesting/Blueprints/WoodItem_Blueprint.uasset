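; Stackable VR wood pickup that shows its count in a TextRender and lets motion controllers split the stack.
; Overlapping wood items merge counts and destroy the absorbed actor.
; Gates opened by trigger or face button let grip spawn a hand-attached piece, removing one or halving the stack respectively.
; Splitting clears CanBeStacked, restored after a delay if wood above one remains, with logic duplicated per hand.
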(event `self.WoodMesh.OnComponentBeginOverlap`
  (params (OverlappedComponent :type "PrimitiveComponent Object Reference") (OtherActor :type "Actor Object Reference") (OtherComp :type "PrimitiveComponent Object Reference") (OtherBodyIndex :type Integer) (bFromSweep :type Boolean) (SweepResult :type "HitResult Structure (by ref)"))
  (bind _amountofwood (`self.AmountOfWood`))
  ;[1 1 1] Increment amount of wood
  (if (== "WoodItem_Blueprint_C" (`GameplayStatics.GetObjectClass` OtherActor))
    (bind _aswood_item_blueprint (cast `/Game/AliTesting/Blueprints/WoodItem_Blueprint` OtherActor))
    (if (`/Game/AliTesting/Blueprints/WoodItem_Blueprint.CanBeStacked` _aswood_item_blueprint)
      (if (<= _amountofwood 100)
        (bind _output_get (set `self.AmountOfWood` (+ (`/Game/AliTesting/Blueprints/WoodItem_Blueprint.AmountOfWood` _aswood_item_blueprint) _amountofwood)))
        (`TextRenderComponent.K2_SetText` (`self.TextRender`) (`KismetTextLibrary.Conv_IntToText` _output_get))
        (`self.K2_DestroyActor` _aswood_item_blueprint)))))

(event `Key|MotionController_Right_Grip1` :consume false
  (params (Key :type "Key Structure"))
  (bind _woodmesh (`self.WoodMesh`))
  (bind (_returnvalue_x _returnvalue_y _returnvalue_z) (`KismetMathLibrary.BreakVector` (`SceneComponent.K2_GetComponentLocation` _woodmesh)))
  ;[1 1 1] Stacking physics R - as long as you hold trigger while grabbing a stack of wood, itll pull one wood out of the stack
  (:`Pressed`
    (`/Engine/EditorBlueprintResources/StandardMacros.Gate` true :!label _label
      (:`Exit`
        (bind _ascharacter_blueprint (cast `/Game/AliTesting/Blueprints/Character_Blueprint` (`GameplayStatics.GetPlayerCharacter` 0)))
        (if (`PrimitiveComponent.IsOverlappingComponent` (`/Game/AliTesting/Blueprints/Character_Blueprint.GrabSphereR` _ascharacter_blueprint) _woodmesh)
          (bind _returnvalue (`|SpawnActorFromClass` "WoodItem_Blueprint_C" (`KismetMathLibrary.MakeTransform` (`KismetMathLibrary.MakeVector` (+ _returnvalue_x 50.0) _returnvalue_y _returnvalue_z) (struct) (0.1 0.1 0.1)) "AlwaysSpawn" "OverrideRootScale" null null))
          (set `self.CanBeStacked` false)
          (`self.K2_AttachToComponent` _returnvalue (`/Game/AliTesting/Blueprints/Character_Blueprint.HandSMRight` _ascharacter_blueprint) "None" "SnapToTarget" "KeepRelative" "KeepWorld" true)
          (bind _output_get (set `self.AmountOfWood` (- (`self.AmountOfWood`) 1)))
          (if (> _output_get 1)
            (`TextRenderComponent.K2_SetText` (`self.TextRender`) (`KismetTextLibrary.Conv_IntToText` _output_get))
            (`KismetSystemLibrary.Delay` 5.0)
            (set `self.CanBeStacked` true)))))))

(event `Key|MotionController_Right_Trigger` :consume false
  (params (Key :type "Key Structure"))
  ;[1 1 1] Stacking physics R - as long as you hold trigger while grabbing a stack of wood, itll pull one wood out of the stack
  (:`Pressed`
    (if (> (`self.AmountOfWood`) 1)
      (goto _label :!via `Open`)))
  (:`Released`
    (goto _label :!via `Close`)))

(event `Key|MotionController_Right_Grip1` :consume false
  (params (Key :type "Key Structure"))
  (bind _woodmesh (`self.WoodMesh`))
  (bind _amountofwood (`self.AmountOfWood`))
  (bind (_returnvalue_x _returnvalue_y _returnvalue_z) (`KismetMathLibrary.BreakVector` (`SceneComponent.K2_GetComponentLocation` _woodmesh)))
  (bind _returnvalue (/ _amountofwood 2))
  ;[1 1 1] Stacking physics R - as long as you hold trigger while grabbing a stack of wood, itll pull one wood out of the stack
  (:`Pressed`
    (`/Engine/EditorBlueprintResources/StandardMacros.Gate` true :!label _label_2
      (:`Exit`
        (bind _ascharacter_blueprint (cast `/Game/AliTesting/Blueprints/Character_Blueprint` (`GameplayStatics.GetPlayerCharacter` 0)))
        (if (`PrimitiveComponent.IsOverlappingComponent` (`/Game/AliTesting/Blueprints/Character_Blueprint.GrabSphereR` _ascharacter_blueprint) _woodmesh)
          (bind _returnvalue_2 (`|SpawnActorFromClass` "WoodItem_Blueprint_C" (`KismetMathLibrary.MakeTransform` (`KismetMathLibrary.MakeVector` (+ _returnvalue_x 50.0) _returnvalue_y _returnvalue_z) (struct) (0.1 0.1 0.1)) "AlwaysSpawn" "OverrideRootScale" null null))
          (set `self.CanBeStacked` false)
          (`self.K2_AttachToComponent` _returnvalue_2 (`/Game/AliTesting/Blueprints/Character_Blueprint.HandSMRight` _ascharacter_blueprint) "None" "SnapToTarget" "KeepRelative" "KeepWorld" true)
          (bind _output_get (set `self.AmountOfWood` _returnvalue))
          (if (!= (mod _amountofwood 2) 0)
            (bind _result (`/Engine/EditorBlueprintResources/StandardMacros.IncrementInt` _returnvalue)
              (:`  `
                (set `/Game/AliTesting/Blueprints/WoodItem_Blueprint.AmountOfWood` _result _returnvalue_2)))
            (else
              (set `/Game/AliTesting/Blueprints/WoodItem_Blueprint.AmountOfWood` _returnvalue _returnvalue_2)))
          (if (> _output_get 1)
            (`TextRenderComponent.K2_SetText` (`self.TextRender`) (`KismetTextLibrary.Conv_IntToText` _output_get))
            (`TextRenderComponent.K2_SetText` (`/Game/AliTesting/Blueprints/WoodItem_Blueprint.TextRender` _returnvalue_2) (`KismetTextLibrary.Conv_IntToText` (`/Game/AliTesting/Blueprints/WoodItem_Blueprint.AmountOfWood` _returnvalue_2)))
            (`KismetSystemLibrary.Delay` 0.5)
            (set `self.CanBeStacked` true)))))))

(event `Key|MotionController_Right_FaceButton1` :consume false
  (params (Key :type "Key Structure"))
  ;[1 1 1] Stacking physics R - as long as you hold trigger while grabbing a stack of wood, itll pull one wood out of the stack
  (:`Pressed`
    (if (> (`self.AmountOfWood`) 1)
      (goto _label_2 :!via `Open`)))
  (:`Released`
    (goto _label_2 :!via `Close`)))

(event `Key|MotionController_Left_Grip1` :consume false
  (params (Key :type "Key Structure"))
  (bind _woodmesh (`self.WoodMesh`))
  (bind (_returnvalue_x _returnvalue_y _returnvalue_z) (`KismetMathLibrary.BreakVector` (`SceneComponent.K2_GetComponentLocation` _woodmesh)))
  ;[1 1 1] Stacking physics L - as long as you hold trigger while grabbing a stack of wood, itll pull one wood out of the stack
  (:`Pressed`
    (`/Engine/EditorBlueprintResources/StandardMacros.Gate` true :!label _label_3
      (:`Exit`
        (bind _ascharacter_blueprint (cast `/Game/AliTesting/Blueprints/Character_Blueprint` (`GameplayStatics.GetPlayerCharacter` 0)))
        (if (`PrimitiveComponent.IsOverlappingComponent` (`/Game/AliTesting/Blueprints/Character_Blueprint.GrabSphereL` _ascharacter_blueprint) _woodmesh)
          (bind _returnvalue (`|SpawnActorFromClass` "WoodItem_Blueprint_C" (`KismetMathLibrary.MakeTransform` (`KismetMathLibrary.MakeVector` (+ _returnvalue_x 50.0) _returnvalue_y _returnvalue_z) (struct) (0.1 0.1 0.1)) "AlwaysSpawn" "OverrideRootScale" null null))
          (set `self.CanBeStacked` false)
          (`self.K2_AttachToComponent` _returnvalue (`/Game/AliTesting/Blueprints/Character_Blueprint.HandSMLeft` _ascharacter_blueprint) "None" "SnapToTarget" "KeepRelative" "KeepWorld" true)
          (bind _output_get (set `self.AmountOfWood` (- (`self.AmountOfWood`) 1)))
          (if (> _output_get 1)
            (`TextRenderComponent.K2_SetText` (`self.TextRender`) (`KismetTextLibrary.Conv_IntToText` _output_get))
            (`KismetSystemLibrary.Delay` 5.0)
            (set `self.CanBeStacked` true)))))))

(event `Key|MotionController_Left_Trigger` :consume false
  (params (Key :type "Key Structure"))
  ;[1 1 1] Stacking physics L - as long as you hold trigger while grabbing a stack of wood, itll pull one wood out of the stack
  (:`Pressed`
    (if (> (`self.AmountOfWood`) 1)
      (goto _label_3 :!via `Open`)))
  (:`Released`
    (goto _label_3 :!via `Close`)))

(event `Key|MotionController_Left_Grip1` :consume false
  (params (Key :type "Key Structure"))
  (bind _amountofwood (`self.AmountOfWood`))
  (bind _woodmesh (`self.WoodMesh`))
  (bind _returnvalue (/ _amountofwood 2))
  (bind (_returnvalue_x _returnvalue_y _returnvalue_z) (`KismetMathLibrary.BreakVector` (`SceneComponent.K2_GetComponentLocation` _woodmesh)))
  ;[1 1 1] Stacking physics L - as long as you hold trigger while grabbing a stack of wood, itll pull one wood out of the stack
  (:`Pressed`
    (`/Engine/EditorBlueprintResources/StandardMacros.Gate` true :!label _label_4
      (:`Exit`
        (bind _ascharacter_blueprint (cast `/Game/AliTesting/Blueprints/Character_Blueprint` (`GameplayStatics.GetPlayerCharacter` 0)))
        (if (`PrimitiveComponent.IsOverlappingComponent` (`/Game/AliTesting/Blueprints/Character_Blueprint.GrabSphereL` _ascharacter_blueprint) _woodmesh)
          (bind _returnvalue_2 (`|SpawnActorFromClass` "WoodItem_Blueprint_C" (`KismetMathLibrary.MakeTransform` (`KismetMathLibrary.MakeVector` (+ _returnvalue_x 50.0) _returnvalue_y _returnvalue_z) (struct) (0.1 0.1 0.1)) "AlwaysSpawn" "OverrideRootScale" null null))
          (set `self.CanBeStacked` false)
          (`self.K2_AttachToComponent` _returnvalue_2 (`/Game/AliTesting/Blueprints/Character_Blueprint.HandSMLeft` _ascharacter_blueprint) "None" "SnapToTarget" "KeepRelative" "KeepWorld" true)
          (bind _output_get (set `self.AmountOfWood` _returnvalue))
          (if (!= (mod _amountofwood 2) 0)
            (bind _result (`/Engine/EditorBlueprintResources/StandardMacros.IncrementInt` _returnvalue)
              (:`  `
                (set `/Game/AliTesting/Blueprints/WoodItem_Blueprint.AmountOfWood` _result _returnvalue_2)
                (if (> _output_get 1)
                  (`TextRenderComponent.K2_SetText` (`self.TextRender`) (`KismetTextLibrary.Conv_IntToText` _output_get))
                  (`TextRenderComponent.K2_SetText` (`/Game/AliTesting/Blueprints/WoodItem_Blueprint.TextRender` _returnvalue_2) (`KismetTextLibrary.Conv_IntToText` (`/Game/AliTesting/Blueprints/WoodItem_Blueprint.AmountOfWood` _returnvalue_2)))
                  (`KismetSystemLibrary.Delay` 0.5)
                  (set `self.CanBeStacked` true))))))))))

(event `Key|MotionController_Left_FaceButton1` :consume false
  (params (Key :type "Key Structure"))
  ;[1 1 1] Stacking physics L - as long as you hold trigger while grabbing a stack of wood, itll pull one wood out of the stack
  (:`Pressed`
    (if (> (`self.AmountOfWood`) 1)
      (goto _label_4 :!via `Open`)))
  (:`Released`
    (goto _label_4 :!via `Close`)))

(fn `UserConstructionScript`)