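; Hand-held ice pick for motion-controller climbing, reacting when its PickHead overlaps the ClimbingWall_Blueprint.
; If the pick faces the wall's origin within 45 degrees, it checks each of the player character's hands for itself.
; While held, it adds movement input along the wall-to-controller direction and zeroes that hand mesh's physics velocity.
; These while loops have no delay, so they never yield to the next frame.
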(event `self.PickHead.OnComponentBeginOverlap`
  (params (OverlappedComponent :type "PrimitiveComponent Object Reference") (OtherActor :type "Actor Object Reference") (OtherComp :type "PrimitiveComponent Object Reference") (OtherBodyIndex :type Integer) (bFromSweep :type Boolean) (SweepResult :type "HitResult Structure (by ref)"))
  (bind _returnvalue (`self.K2_GetActorLocation` OtherActor))
  (bind _returnvalue_2 (`GameplayStatics.GetPlayerCharacter` 0))
  (bind _icepick (`self.IcePick`))
  (if (== OtherActor "/Game/AliTesting/Blueprints/ClimbingWall_Blueprint.ClimbingWall_Blueprint")
    (if (== (`SceneComponent.K2_GetComponentRotation` _icepick) (`KismetMathLibrary.FindLookAtRotation` (`SceneComponent.K2_GetComponentLocation` _icepick) (`self.K2_GetActorLocation` OtherActor)) :`ErrorTolerance` 45.0)
      (`|ExecutionSequence`
        (:`then_0`
          (bind _ascharacter_blueprint (cast `/Game/AliTesting/Blueprints/Character_Blueprint` _returnvalue_2))
          (while (== (`/Game/AliTesting/Blueprints/Character_Blueprint.HeldComponentL` _ascharacter_blueprint) self)
            (`Pawn.AddMovementInput` _ascharacter_blueprint (`KismetMathLibrary.Normal` (- (`SceneComponent.K2_GetComponentLocation` (`/Game/AliTesting/Blueprints/Character_Blueprint.MC_Left` _ascharacter_blueprint)) _returnvalue)) 1.0 false)
            ;[1 1 1] will this freeze the pick
            (`PrimitiveComponent.SetPhysicsLinearVelocity` (`/Game/AliTesting/Blueprints/Character_Blueprint.HandSMLeft` _ascharacter_blueprint) (0.0 0.0 0.0) false "None")))
        (:`then_1`
          (bind _ascharacter_blueprint_2 (cast `/Game/AliTesting/Blueprints/Character_Blueprint` _returnvalue_2))
          (while (== (`/Game/AliTesting/Blueprints/Character_Blueprint.HeldComponentR` _ascharacter_blueprint_2) self)
            (`Pawn.AddMovementInput` _ascharacter_blueprint_2 (`KismetMathLibrary.Normal` (- (`SceneComponent.K2_GetComponentLocation` (`/Game/AliTesting/Blueprints/Character_Blueprint.MC_Right` _ascharacter_blueprint_2)) _returnvalue)) 1.0 false)
            (`PrimitiveComponent.SetPhysicsLinearVelocity` (`/Game/AliTesting/Blueprints/Character_Blueprint.HandSMRight` _ascharacter_blueprint_2) (0.0 0.0 0.0) false "None")))))))

(fn `UserConstructionScript`)