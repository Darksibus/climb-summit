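; VR backpack that the player takes off, puts back on and stores held objects in, using either motion controller grip.
; Grip press or release with a grab sphere in the character's pack collision detaches or attaches it at PackAttachmentPoint.
; Releasing a held component inside runs a shared shrink timeline, then attaches it, though the right-hand branch parents PackSM to the item.
; Gripping a stored component detaches it and reverses the timeline.
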(event `Key|MotionController_Right_Grip1` :consume false
  (params (Key :type "Key Structure"))
  ;[1 1 1] Take off pack and put it on
  (:`Pressed`
    (bind _returnvalue (`PrimitiveComponent.IsOverlappingComponent` (`/Game/AliTesting/Blueprints/Character_Blueprint.GrabSphereR` (stale _ascharacter_blueprint)) (`/Game/AliTesting/Blueprints/Character_Blueprint.PackCollision` (stale _ascharacter_blueprint))))
    (if _returnvalue
      (`self.K2_DetachFromActor` "KeepRelative")))
  (:`Released`
    (bind _ascharacter_blueprint (cast `/Game/AliTesting/Blueprints/Character_Blueprint` (`GameplayStatics.GetPlayerCharacter` 0)))
    (if _returnvalue
      (`self.K2_AttachToComponent` (`/Game/AliTesting/Blueprints/Character_Blueprint.PackAttachmentPoint` _ascharacter_blueprint) "None" "SnapToTarget" "SnapToTarget" "KeepRelative"))))

(event `Key|MotionController_Right_Grip1` :consume false
  (params (Key :type "Key Structure"))
  (bind _packsm (`self.PackSM`))
  ;[1 1 1] Putting stuff inside & taking it out
  (:`Pressed`
    (if (stale `Key|MotionController_Right_Grip1` _returnvalue_4)
      (if (`PrimitiveComponent.IsOverlappingComponent` (stale _asprimitive_component) (`/Game/AliTesting/Blueprints/Character_Blueprint.GrabSphereR` (stale _ascharacter_blueprint)))
        (`SceneComponent.K2_DetachFromComponent` (stale _asprimitive_component) "KeepRelative" "KeepRelative" "KeepRelative" true)
        (`TimelineComponent.ReverseFromEnd` (`self.LerpTimeline`))
        (bind _returnvalue (`SceneComponent.K2_GetComponentLocation` (stale _asprimitive_component)))
        (bind _returnvalue_2 (`KismetMathLibrary.TLerp` (`KismetMathLibrary.Conv_VectorToTransform` _returnvalue) (`KismetMathLibrary.MakeTransform` (- _returnvalue (`SceneComponent.K2_GetComponentLocation` (`/Game/AliTesting/Blueprints/Character_Blueprint.PackAttachmentPoint` (stale _ascharacter_blueprint)))) (struct) (0.1 0.1 0.1)) (stale `Key|MotionController_Right_Grip1` _alpha_lerp)))
        (`SceneComponent.K2_SetWorldTransform` (stale _asprimitive_component) _returnvalue_2 false false)
        (`PrimitiveComponent.SetCollisionResponseToChannel` (stale _asprimitive_component) "ECC_WorldStatic" "ECR_Overlap"))))
  (:`Released`
    (if (`PrimitiveComponent.IsOverlappingComponent` (`self.PackCollision`) (`/Game/AliTesting/Blueprints/Character_Blueprint.GrabSphereR` (stale _ascharacter_blueprint)))
      (bind _asprimitive_component (cast `PrimitiveComponent` (`/Game/AliTesting/Blueprints/Character_Blueprint.HeldComponentR` (stale _ascharacter_blueprint))))
      (if (`PrimitiveComponent.IsOverlappingComponent` (`self.PackCollision`) _asprimitive_component)
        (bind (_direction _alpha_lerp) (`Timeline|LerpTimeline` :!via `PlayFromStart` :!label _label)
          (:`Update`
            (`|ExecutionSequence`
              (:`then_0`
                (`SceneComponent.K2_SetWorldTransform` _asprimitive_component _returnvalue_2 false false))
              (:`then_1`
                (bind _returnvalue_3 (`SceneComponent.K2_GetComponentLocation` (stale _asprimitive_component)))
                (`SceneComponent.K2_SetWorldTransform` (stale _asprimitive_component) (`KismetMathLibrary.TLerp` (`KismetMathLibrary.Conv_VectorToTransform` _returnvalue_3) (`KismetMathLibrary.MakeTransform` (- _returnvalue_3 (`SceneComponent.K2_GetComponentLocation` (`/Game/AliTesting/Blueprints/Character_Blueprint.PackAttachmentPoint` (stale _ascharacter_blueprint)))) (struct) (0.1 0.1 0.1)) _alpha_lerp) false false))))
          (:`Finished`
            (`|ExecutionSequence`
              (:`then_0`
                (bind _returnvalue_4 (`SceneComponent.K2_AttachToComponent` _packsm _asprimitive_component "None" "KeepRelative" "KeepRelative" "KeepRelative" true))
                (`PrimitiveComponent.SetCollisionResponseToChannel` _asprimitive_component "ECC_GameTraceChannel3" "ECR_Ignore"))
              (:`then_1`
                (`SceneComponent.K2_AttachToComponent` (stale _asprimitive_component) _packsm "None" "KeepRelative" "KeepRelative" "KeepRelative" true)
                (`PrimitiveComponent.SetCollisionResponseToChannel` (stale _asprimitive_component) "ECC_GameTraceChannel3" "ECR_Ignore")))))))))

(event `Key|MotionController_Left_Grip1` :consume false
  (params (Key :type "Key Structure"))
  ;[1 1 1] Putting stuff inside & taking it out
  (:`Pressed`
    (if (stale `Key|MotionController_Right_Grip1` _returnvalue_4)
      (if (`PrimitiveComponent.IsOverlappingComponent` (stale _asprimitive_component) (`/Game/AliTesting/Blueprints/Character_Blueprint.GrabSphereL` (stale _ascharacter_blueprint)))
        (`SceneComponent.K2_DetachFromComponent` (stale _asprimitive_component) "KeepRelative" "KeepRelative" "KeepRelative" true)
        (`TimelineComponent.ReverseFromEnd` (`self.LerpTimeline`))
        (bind _returnvalue (`SceneComponent.K2_GetComponentLocation` (stale _asprimitive_component)))
        (`SceneComponent.K2_SetWorldTransform` (stale _asprimitive_component) (`KismetMathLibrary.TLerp` (`KismetMathLibrary.Conv_VectorToTransform` _returnvalue) (`KismetMathLibrary.MakeTransform` (- _returnvalue (`SceneComponent.K2_GetComponentLocation` (`/Game/AliTesting/Blueprints/Character_Blueprint.PackAttachmentPoint` (stale _ascharacter_blueprint)))) (struct) (0.1 0.1 0.1)) (stale `Key|MotionController_Right_Grip1` _alpha_lerp)) false false)
        (`PrimitiveComponent.SetCollisionResponseToChannel` (stale _asprimitive_component) "ECC_GameTraceChannel2" "ECR_Overlap"))))
  (:`Released`
    (if (`PrimitiveComponent.IsOverlappingComponent` (`self.PackCollision`) (`/Game/AliTesting/Blueprints/Character_Blueprint.GrabSphereL` (stale _ascharacter_blueprint)))
      (bind _asprimitive_component (cast `PrimitiveComponent` (`/Game/AliTesting/Blueprints/Character_Blueprint.HeldComponentL` (stale _ascharacter_blueprint))))
      (if (`PrimitiveComponent.IsOverlappingComponent` (`self.PackCollision`) _asprimitive_component)
        (goto _label :!via `PlayFromStart`)))))

(event `Key|MotionController_Left_Grip1` :consume false
  (params (Key :type "Key Structure"))
  ;[1 1 1] Take off pack and put it on
  (:`Pressed`
    (bind _returnvalue (`PrimitiveComponent.IsOverlappingComponent` (`/Game/AliTesting/Blueprints/Character_Blueprint.GrabSphereL` (stale _ascharacter_blueprint)) (`/Game/AliTesting/Blueprints/Character_Blueprint.PackCollision` (stale _ascharacter_blueprint))))
    (if _returnvalue
      (`self.K2_DetachFromActor` "KeepRelative")))
  (:`Released`
    (bind _ascharacter_blueprint (cast `/Game/AliTesting/Blueprints/Character_Blueprint` (`GameplayStatics.GetPlayerCharacter` 0)))
    (if _returnvalue
      (`self.K2_AttachToComponent` (`/Game/AliTesting/Blueprints/Character_Blueprint.PackAttachmentPoint` _ascharacter_blueprint) "None" "SnapToTarget" "SnapToTarget" "KeepRelative"))))

(fn `UserConstructionScript`)