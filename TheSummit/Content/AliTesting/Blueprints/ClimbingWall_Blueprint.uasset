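; Climbing wall test Blueprint with ten hold spheres, which it gathers into an array on BeginPlay.
; Unconnected left and right climbing logic checks whether the player's grab sphere overlaps the first hold only.
; It would force movement input along the motion-controller-to-hold direction and pause that hand mesh's tick, with separate chains to re-enable it.
; None of this climbing logic runs, and a note suggests moving it to the character Blueprint.
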(event `Key|MotionController_Right_Grip1` :consume false
  (params (Key :type "Key Structure"))
  ;[1 1 1] It'd probably be a good idea to just transfer these to the character blueprint - later tho
  ;;[1 1 1] Climbing Right
)

(event `Key|MotionController_Left_Grip1` :consume false
  (params (Key :type "Key Structure"))
  ;[1 1 1] It'd probably be a good idea to just transfer these to the character blueprint - later tho
  ;;[1 1 1] ClimbingLeft
)

(event `self.ReceiveBeginPlay`
  (set `self.holdSphere array` (`|MakeArray` (`self.holdSphere0`) (`self.holdSphere1`) (`self.holdSphere2`) (`self.holdSphere3`) (`self.holdSphere4`) (`self.holdSphere5`) (`self.holdSphere6`) (`self.holdSphere7`) (`self.holdSphere8`) (`self.holdSphere9`) :!type "SceneComponent Object Reference")))

(fn `UserConstructionScript`)