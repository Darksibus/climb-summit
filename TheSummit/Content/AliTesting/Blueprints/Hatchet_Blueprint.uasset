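; Hatchet weapon Blueprint that damages actors its axe head hits.
; When AxeHead begins an overlap, it compares the static mesh's world rotation to the look-at rotation toward the other actor, within an angular tolerance.
; If they match and the axe head's physics velocity meets a minimum speed, it applies damage.
; An unconnected chain that briefly disables component tick never runs.
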(event `self.AxeHead.OnComponentBeginOverlap`
  (params (OverlappedComponent :type "PrimitiveComponent Object Reference") (OtherActor :type "Actor Object Reference") (OtherComp :type "PrimitiveComponent Object Reference") (OtherBodyIndex :type Integer) (bFromSweep :type Boolean) (SweepResult :type "HitResult Structure (by ref)"))
  (bind _staticmeshcomponent (`self.StaticMeshComponent`))
  (bind (_returnvalue_roll _returnvalue_pitch _returnvalue_yaw) (`KismetMathLibrary.BreakRotator` (`KismetMathLibrary.FindLookAtRotation` (`SceneComponent.K2_GetComponentLocation` _staticmeshcomponent) (`self.K2_GetActorLocation` OtherActor))))
  (if (== (`KismetMathLibrary.MakeRotator` _returnvalue_roll _returnvalue_pitch _returnvalue_yaw) (`SceneComponent.K2_GetComponentRotation` _staticmeshcomponent) :`ErrorTolerance` 30.0)
    (bind _returnvalue (`PrimitiveComponent.GetPhysicsLinearVelocity` (`self.AxeHead`) "None"))
    (if (>= (`KismetMathLibrary.VSize` _returnvalue) 5.0)
      (`GameplayStatics.ApplyDamage` OtherActor 1.0))))

(fn `UserConstructionScript`)